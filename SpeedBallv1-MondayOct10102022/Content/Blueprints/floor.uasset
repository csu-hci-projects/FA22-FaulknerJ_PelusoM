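; Floor actor that acts as a kill zone for the ball game, costing a life when any actor overlaps it.
; While more than one life remains in the GIDemo game instance, it reopens Level_BallGame_1 and decrements Lives, which persists across the reload.
; Otherwise it pauses the game, shows the mouse cursor and adds a DeathMenu widget to the viewport.
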(event `self.ReceiveActorBeginOverlap`
  (params (OtherActor :type "Actor Object Reference"))
  (bind _asgidemo (cast `/Game/Blueprints/GIDemo` (`GameplayStatics.GetGameInstance`)))
  (if (> (`/Game/Blueprints/GIDemo.Lives` _asgidemo) 1)
    (`GameplayStatics.OpenLevelBySoftObjectPtr` "/Game/Maps/Level_BallGame_1.Level_BallGame_1")
    (bind _asgidemo_2 (cast `/Game/Blueprints/GIDemo` (`GameplayStatics.GetGameInstance`)))
    (set `/Game/Blueprints/GIDemo.Lives` (- (`/Game/Blueprints/GIDemo.Lives` _asgidemo_2) 1) _asgidemo_2)
    (else
      (`GameplayStatics.SetGamePaused` true)
      (set `PlayerController.bShowMouseCursor` true (`GameplayStatics.GetPlayerController` 0))
      (bind _returnvalue (`|CreateWidget` "/Game/Blueprints/UI/DeathMenu.DeathMenu_C"))
      (`UserWidget.AddToViewport` _returnvalue 0))))

(fn `UserConstructionScript`)
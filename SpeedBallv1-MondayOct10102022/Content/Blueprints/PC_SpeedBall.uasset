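; Player controller for a rolling-ball game that sets up the UI, drives the ball and handles the end of the game.
; BeginPlay resets the GameInstance key count, adds the HUD and briefly shows an intro widget.
; Move axes apply torque to the ball fetched from the pawn via GetBallRefMessage, while mouse Y pitches the camera.
; Tick polls EndTheGame, then after a short delay pauses and shows the end menu with the cursor.
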(event `self.ReceiveBeginPlay`
  (bind _asgidemo (cast `/Game/Blueprints/GIDemo` (`GameplayStatics.GetGameInstance`)))
  (set `/Game/Blueprints/GIDemo.KeyNum` 0 _asgidemo)
  (bind _returnvalue (`|CreateWidget` "/Game/Blueprints/UI/HUD.HUD_C"))
  (`UserWidget.AddToViewport` _returnvalue 0)
  (bind _returnvalue_2 (`|CreateWidget` "/Game/Blueprints/UI/Beginning.Beginning_C"))
  (`UserWidget.AddToViewport` _returnvalue_2 0)
  (`KismetSystemLibrary.Delay` 2.0)
  (`Widget.RemoveFromParent` _returnvalue_2))

(event `InputAxis|MouseY`
  (params (AxisValue :type "Float (single-precision)"))
  ;[1 1 1] Camera
  (`Pawn.AddControllerPitchInput` (`GameplayStatics.GetPlayerPawn` 0) AxisValue))

(event `InputAxis|MoveX_RL`
  (params (AxisValue :type "Float (single-precision)"))
  (bind _ball (message `/Game/Blueprints/Interfaces/IBP_BPBall.GetBallRef` (`GameplayStatics.GetPlayerPawn` 0)))
  (bind _ball_2 (`/Game/Blueprints/BP_Ball.Ball` _ball)
    (:`then`
      (`PrimitiveComponent.AddTorqueInRadians` _ball_2 (`KismetMathLibrary.MakeVector` (* AxisValue 20.0)) "None" true))
    (:`else`)))

(event `End Game`
  (`GameplayStatics.SetGamePaused` true)
  (set `PlayerController.bShowMouseCursor` true (`GameplayStatics.GetPlayerController` 0))
  (bind _returnvalue (`|CreateWidget` "/Game/Blueprints/UI/EndMenu.EndMenu_C"))
  (`UserWidget.AddToViewport` _returnvalue 0))

(event `InputAxis|MoveY_FB`
  (params (AxisValue :type "Float (single-precision)"))
  (bind _ball (message `/Game/Blueprints/Interfaces/IBP_BPBall.GetBallRef` (`GameplayStatics.GetPlayerPawn` 0)))
  (bind _ball_2 (`/Game/Blueprints/BP_Ball.Ball` _ball)
    (:`then`
      (`PrimitiveComponent.AddTorqueInRadians` _ball_2 (`KismetMathLibrary.MakeVector` 0.0 (* AxisValue 20.0)) "None" true))
    (:`else`)))

(event `Check Goal`
  (if (`self.EndTheGame`)
    (`KismetSystemLibrary.Delay` 0.25)
    (`self.End Game`)))

(event `self.ReceiveTick`
  (params (DeltaSeconds :type "Float (single-precision)"))
  (`self.Check Goal`))

(fn `UserConstructionScript`)
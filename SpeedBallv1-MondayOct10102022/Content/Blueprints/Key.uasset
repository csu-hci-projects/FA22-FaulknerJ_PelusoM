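; Key pickup actor that the player collects to raise a persistent key count.
; On overlap with an actor tagged Player, it destroys itself and increments KeyNum on the GIDemo game instance.
; Tick spins it slowly around its yaw axis using a delta-time-scaled local rotation.
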(event `self.ReceiveActorBeginOverlap`
  (params (OtherActor :type "Actor Object Reference"))
  (if (`self.ActorHasTag` OtherActor "Player")
    (`self.K2_DestroyActor`)
    (bind _asgidemo (cast `/Game/Blueprints/GIDemo` (`GameplayStatics.GetGameInstance`)))
    (set `/Game/Blueprints/GIDemo.KeyNum` (+ (`/Game/Blueprints/GIDemo.KeyNum` _asgidemo) 1) _asgidemo)))

(event `self.ReceiveTick`
  (params (DeltaSeconds :type "Float (single-precision)"))
  (`self.K2_AddActorLocalRotation` (`KismetMathLibrary.MakeRotator` 0.0 0.0 (* DeltaSeconds 20.0))))

(fn `UserConstructionScript`)
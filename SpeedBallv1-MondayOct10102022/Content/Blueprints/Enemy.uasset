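; Enemy is a hazard actor that spins in place and damages the player on contact.
; On any overlap it plays an explosion sound, destroys itself, and subtracts one from PlayerHealth in the GIDemo game instance, without checking what overlapped it.
; Each Tick it yaws at a frame-rate-independent speed scaled by the game instance's DifficultyModifier.
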(event `self.ReceiveActorBeginOverlap`
  (params (OtherActor :type "Actor Object Reference"))
  (`GameplayStatics.PlaySoundAtLocation` "/Game/SuperGrid/TutorialLevel/SoundEffects/Cue_Explosions.Cue_Explosions" (`self.K2_GetActorLocation`) (struct) 1.0 1.0 0.0 null null null null)
  (`self.K2_DestroyActor`)
  (bind _asgidemo (cast `/Game/Blueprints/GIDemo` (`GameplayStatics.GetGameInstance`)))
  (set `/Game/Blueprints/GIDemo.PlayerHealth` (- (`/Game/Blueprints/GIDemo.PlayerHealth` _asgidemo) 1.0) _asgidemo))

(event `self.ReceiveTick`
  (params (DeltaSeconds :type "Float (single-precision)"))
  (bind _asgidemo (cast `/Game/Blueprints/GIDemo` (`GameplayStatics.GetGameInstance`)))
  (`self.K2_AddActorLocalRotation` (`KismetMathLibrary.MakeRotator` 0.0 0.0 (* (* DeltaSeconds 50.0) (`/Game/Blueprints/GIDemo.Difficulty_modifier` _asgidemo)))))

(fn `UserConstructionScript`)
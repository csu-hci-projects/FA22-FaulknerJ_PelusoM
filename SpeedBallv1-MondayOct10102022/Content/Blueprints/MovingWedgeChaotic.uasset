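; MovingWedgeChaotic is a moving wedge actor that shuttles back and forth along a horizontal line.
; Each tick it offsets itself along the 2D-normalized Direction, scaled by Speed and delta time, without sweeping for collisions.
; A looping timer set on BeginPlay negates Direction every DirectionChange seconds to reverse the motion.
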(event `self.ReceiveBeginPlay`
  (`KismetSystemLibrary.K2_SetTimerDelegate` (delegate `change direction`) (`self.Direction Change`) true))

(event `change direction`
  (set `self.Direction ` (* (`self.Direction `) -1.0)))

(event `self.ReceiveTick`
  (params (DeltaSeconds :type "Float (single-precision)"))
  (`self.K2_AddActorWorldOffset` (* (`KismetMathLibrary.Vector_Normal2D` (`self.Direction `)) (* (`self.Speed`) (`GameplayStatics.GetWorldDeltaSeconds`)))))

(fn `UserConstructionScript`)